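; BP_TowerPlace is a clickable build spot where the player places towers while the game mode's IsBreak is true.
; Hovering during a break swaps the Place component's material to crystal, and leaving restores smooth stone.
; A click spawns the player controller's selected Tower class above the spot, then passes its Price to the controller's Buy.
; A successful purchase plays a hammer sound, while a failed one destroys the just-spawned tower.
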(event `self.Place.OnBeginCursorOver`
  (params (TouchedComponent :type "PrimitiveComponent Object Reference"))
  (bind _asbp_my_game_mode (cast `/Game/Blueprints/Core/BP_MyGameMode` (`GameplayStatics.GetGameMode`)))
  (if (`/Game/Blueprints/Core/BP_MyGameMode.IsBreak` _asbp_my_game_mode)
    (`PrimitiveComponent.SetMaterial` TouchedComponent 0 "/Game/Assets/Objects/Crystal/M_Crystal.M_Crystal")))

(event `self.Place.OnEndCursorOver`
  (params (TouchedComponent :type "PrimitiveComponent Object Reference"))
  (`PrimitiveComponent.SetMaterial` TouchedComponent 0 "/Game/Assets/Objects/Crystal/M_SmoothStone.M_SmoothStone"))

(event `self.Place.OnClicked`
  (params (TouchedComponent :type "PrimitiveComponent Object Reference") (ButtonPressed :type "Key Structure"))
  (bind _asbp_my_game_mode (cast `/Game/Blueprints/Core/BP_MyGameMode` (`GameplayStatics.GetGameMode`)))
  (if (`/Game/Blueprints/Core/BP_MyGameMode.IsBreak` _asbp_my_game_mode)
    (bind _asbp_my_player_controller (cast `/Game/Blueprints/Core/BP_MyPlayerController` (`GameplayStatics.GetPlayerController` 0)))
    (bind _astower (castclass `Tower` (`|ConvertAsset` (`/Game/Blueprints/Core/BP_MyPlayerController.StructureSelected` _asbp_my_player_controller))))
    (bind _returnvalue (`|SpawnActorFromClass` _astower (`KismetMathLibrary.MakeTransform` (`KismetMathLibrary.MakeVector` (.x (.location (`SceneComponent.K2_GetComponentToWorld` TouchedComponent))) (.y (.location (`SceneComponent.K2_GetComponentToWorld` TouchedComponent))) (+ (.z (.location (`SceneComponent.K2_GetComponentToWorld` TouchedComponent))) 100.0)) (.rotation (`SceneComponent.K2_GetComponentToWorld` TouchedComponent)) (1.1 1.1 1.1)) "Undefined" "MultiplyWithRoot" null null))
    (bind _asbp_my_player_controller_2 (cast `/Game/Blueprints/Core/BP_MyPlayerController` (`GameplayStatics.GetPlayerController` 0)))
    (bind _isdone (`/Game/Blueprints/Core/BP_MyPlayerController.Buy` _asbp_my_player_controller_2 (`/Game/Blueprints/Actor/Towers/BP_Tower1.Price` _returnvalue)))
    (if _isdone
      (`GameplayStatics.PlaySoundAtLocation` "/Game/Assets/Sounds/hammer.hammer" (0.0 0.0 0.0) (struct) 0.5 1.0 0.0 null null null null)
      (else
        (`self.K2_DestroyActor` _returnvalue)))))

(fn `UserConstructionScript`)