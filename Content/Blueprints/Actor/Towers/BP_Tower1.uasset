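; BP_Tower1 is a selectable, destructible tower that fires BP_Arrow1 projectiles.
; BeginPlay loads its stats from TowerDataAsset and caches the game mode's round; Shoot spawns an arrow at the barrel carrying the tower's damage.
; Clicking base or barrel sets it as the player controller's TowerSelected after a short delay.
; BP_Fireball overlaps reduce health; death destroys the tower and calls the game mode's OnEnemyKilled, with a zero money award.
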(event `self.ReceiveBeginPlay`
  (bind _towerdataasset (`self.TowerDataAsset`))
  (set `self.ShootDelay` (`TowerData.ShootEachTick` _towerdataasset))
  (bind _output_get (set `self.MaxHealth` (`TowerData.MaxHealth` _towerdataasset)))
  (set `self.Health` _output_get)
  (set `self.Price` (`TowerData.Price` _towerdataasset))
  (set `self.Damages` (`TowerData.Damages` _towerdataasset))
  (set `self.Level` 1)
  (set `self.DetectionSphereRadius` (`TowerData.Scope` _towerdataasset))
  (bind _asbp_my_game_mode (cast `/Game/Blueprints/Core/BP_MyGameMode` (`GameplayStatics.GetGameMode`)))
  (set `self.RoundSetup` (`MyGameMode.Round` _asbp_my_game_mode)))

(event `self.Shoot`
  (bind _returnvalue (`|SpawnActorFromClass` "/Game/Blueprints/Actor/Arrows/BP_Arrow1.BP_Arrow1_C" (`SceneComponent.GetSocketTransform` (`self.BarrelMesh`) "None" "RTS_World") "AlwaysSpawn" "MultiplyWithRoot" null null))
  (set `/Game/Blueprints/Actor/Arrows/BP_Arrow.Damages` (`self.Damages`) _returnvalue))

(event `self.TowerBaseMesh.OnClicked`
  (params (TouchedComponent :type "PrimitiveComponent Object Reference") (ButtonPressed :type "Key Structure"))
  (`KismetSystemLibrary.Delay` 0.2 :!label _label)
  (bind _asbp_my_player_controller (cast `/Game/Blueprints/Core/BP_MyPlayerController` (`GameplayStatics.GetPlayerController` 0)))
  (set `/Game/Blueprints/Core/BP_MyPlayerController.TowerSelected` (`|ConvertAsset` self) _asbp_my_player_controller))

(event `self.BarrelMesh.OnClicked`
  (params (TouchedComponent :type "PrimitiveComponent Object Reference") (ButtonPressed :type "Key Structure"))
  (goto _label))

(event `self.TowerBaseMesh.OnComponentBeginOverlap`
  (params (OverlappedComponent :type "PrimitiveComponent Object Reference") (OtherActor :type "Actor Object Reference") (OtherComp :type "PrimitiveComponent Object Reference") (OtherBodyIndex :type Integer) (bFromSweep :type Boolean) (SweepResult :type "HitResult Structure (by ref)"))
  (bind _asbp_fireball (cast `/Game/Blueprints/Actor/Arrows/BP_Fireball` OtherActor))
  (bind _returnvalue (- (`self.Health`) (`/Game/Blueprints/Actor/Arrows/BP_Fireball.Damages` _asbp_fireball)))
  (if (<= _returnvalue 0.0)
    (`self.K2_DestroyActor` _asbp_fireball)
    (bind _asbp_my_player_controller (cast `/Game/Blueprints/Core/BP_MyPlayerController` (`GameplayStatics.GetPlayerController` 0)))
    (set `/Game/Blueprints/Core/BP_MyPlayerController.Money` (+ (`/Game/Blueprints/Core/BP_MyPlayerController.Money` _asbp_my_player_controller) 0) _asbp_my_player_controller)
    (`self.K2_DestroyActor`)
    (bind _asbp_my_game_mode (cast `/Game/Blueprints/Core/BP_MyGameMode` (`GameplayStatics.GetGameMode`)))
    (`/Game/Blueprints/Core/BP_MyGameMode.OnEnemyKilled` _asbp_my_game_mode)
    (else
      (set `self.Health` _returnvalue)
      (`self.K2_DestroyActor` _asbp_fireball))))

(fn `UserConstructionScript`)