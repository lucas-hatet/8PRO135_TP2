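; BP_Crystal is a destructible crystal that ends the game through BP_MyGameMode when punches deplete its health.
; On a punch at zero health it removes its mesh, waits briefly, calls game over and destroys itself.
; Clicking its sphere during a break while damaged opens a repair confirmation priced by missing health, and accepting restores full health.
; A left mouse press or the assault-start event closes that prompt.
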(event `self.ReceiveBeginPlay`
  (set `self.Health` (`self.MaxHealth`))
  (add `self.OnPunched` (delegate `OnPunched_Event`))
  (bind _asbp_my_game_mode (cast `/Game/Blueprints/Core/BP_MyGameMode` (`GameplayStatics.GetGameMode`)))
  (add `/Game/Blueprints/Core/BP_MyGameMode.OnAssaultStart` _asbp_my_game_mode (delegate `OnAssaultStart`)))

(event `OnPunched_Event`
  (if (<= (`self.Health`) 0)
    (`ActorComponent.K2_DestroyComponent` (`self.StaticMesh`))
    (clear `self.OnPunched`)
    (`KismetSystemLibrary.Delay` 0.5)
    (bind _asbp_my_game_mode (cast `/Game/Blueprints/Core/BP_MyGameMode` (`GameplayStatics.GetGameMode`)))
    (`/Game/Blueprints/Core/BP_MyGameMode.OnGameOver` _asbp_my_game_mode)
    (`self.K2_DestroyActor`)))

(event `OnAccept`
  (set `self.Health` (`self.MaxHealth`)))

(event `self.Sphere.OnClicked`
  (params (TouchedComponent :type "PrimitiveComponent Object Reference") (ButtonPressed :type "Key Structure"))
  (bind _returnvalue (- 2000 (`self.Health`)))
  (`KismetSystemLibrary.Delay` 0.2)
  (bind _asbp_my_game_mode (cast `/Game/Blueprints/Core/BP_MyGameMode` (`GameplayStatics.GetGameMode`)))
  (if (and (> _returnvalue 0) (`/Game/Blueprints/Core/BP_MyGameMode.IsBreak` _asbp_my_game_mode))
    (bind _returnvalue_2 (`|CreateWidget` "/Game/Blueprints/UI/WBP_MessageValidation.WBP_MessageValidation_C"))
    (bind _output_get (set `self.MessageValidationWidget` _returnvalue_2))
    (set `/Game/Blueprints/UI/WBP_MessageValidation.Price` _returnvalue _returnvalue_2)
    (set `/Game/Blueprints/UI/WBP_MessageValidation.Object` "reparer le crystal" _returnvalue_2)
    (`UserWidget.AddToViewport` _output_get 0)
    (`UserWidget.AddToViewport` _returnvalue_2 0)
    (add `/Game/Blueprints/UI/WBP_MessageValidation.OnAccept` _returnvalue_2 (delegate `OnAccept`))))

(event `Key|LeftMouseButton`
  (params (Key :type "Key Structure"))
  (bind _messagevalidationwidget (`self.MessageValidationWidget`))
  (:`Pressed`
    (if (`KismetSystemLibrary.IsValid` _messagevalidationwidget) :!label _label
      (`Widget.RemoveFromParent` _messagevalidationwidget))))

(event `OnAssaultStart`
  (goto _label))

(fn `UserConstructionScript`)