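; Ranged enemy pawn that seeks a prioritized target and shoots fireballs once in range.
; Stats, money drop range and target priorities come from TroopDataAsset, with BP_MyAIController choosing the target.
; A range sphere overlap pins the pawn in place, turns it toward the target and starts a looping fire timer; end overlap resumes seeking and retargets.
; Arrow hits reduce health; death pays the player and notifies the game mode.
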(event `self.ReceiveBeginPlay`
  (bind _troopdataasset (`self.TroopDataAsset`))
  (bind _troopdataasset_2 (`self.TroopDataAsset`))
  (set `self.Speed` (`TroopData.MovementSpeed` _troopdataasset_2))
  (set `self.Health` (`TroopData.MaxHealth` _troopdataasset_2))
  (set `self.Damages` (`TroopData.Damages` _troopdataasset_2))
  (set `self.MoneyDrop` (`KismetMathLibrary.RandomIntegerInRange` (`TroopData.MinMoneyDrop` _troopdataasset_2) (`TroopData.MaxMoneyDrop` _troopdataasset_2)))
  (set `self.StopSeeking` false)
  (`SphereComponent.SetSphereRadius` (`self.Sphere`) 200.0 true)
  (bind _asbp_my_aicontroller (cast `/Game/Blueprints/Core/BP_MyAIController` (`AIBlueprintHelperLibrary.GetAIController` (`self.GetController`))))
  (bind _target (`/Game/Blueprints/Core/BP_MyAIController.ChooseTarget` _asbp_my_aicontroller (`TroopData.FirstTypeTarget` _troopdataasset) (`TroopData.SecondTypeTarget` _troopdataasset) (`TroopData.ThirdTypeTarget` _troopdataasset)))
  (set `self.CurrentTarget` _target))

(event `self.ReceiveTick`
  (params (DeltaSeconds :type "Float (single-precision)"))
  (if (not (`self.StopSeeking`))
    (`self.SeekTargetActor`)
    (else
      (`self.RotateTowardsTarget`)
      (`SceneComponent.K2_SetWorldLocation` (`self.CapsuleComponent`) (`self.LocationToStay`) false false))))

(event `self.CapsuleComponent.OnComponentBeginOverlap`
  (params (OverlappedComponent :type "PrimitiveComponent Object Reference") (OtherActor :type "Actor Object Reference") (OtherComp :type "PrimitiveComponent Object Reference") (OtherBodyIndex :type Integer) (bFromSweep :type Boolean) (SweepResult :type "HitResult Structure (by ref)"))
  (bind _asbp_arrow (cast `/Game/Blueprints/Actor/Arrows/BP_Arrow` OtherActor))
  (bind _output_get (set `self.Health` (- (`self.Health`) (`/Game/Blueprints/Actor/Arrows/BP_Arrow.Damages` _asbp_arrow))))
  (if (<= _output_get 0.0)
    (`self.K2_DestroyActor` _asbp_arrow)
    (`GameplayStatics.PlaySoundAtLocation` "/Game/Assets/Sounds/Arrow/arrow_2.arrow_2" (0.0 0.0 0.0) (struct) 0.1 1.0 0.0 null null null null)
    (bind _asbp_my_player_controller (cast `/Game/Blueprints/Core/BP_MyPlayerController` (`GameplayStatics.GetPlayerController` 0)))
    (set `/Game/Blueprints/Core/BP_MyPlayerController.Money` (+ (`/Game/Blueprints/Core/BP_MyPlayerController.Money` _asbp_my_player_controller) (`self.MoneyDrop`)) _asbp_my_player_controller)
    (`self.K2_DestroyActor`)
    (bind _asbp_my_game_mode (cast `/Game/Blueprints/Core/BP_MyGameMode` (`GameplayStatics.GetGameMode`)))
    (`/Game/Blueprints/Core/BP_MyGameMode.OnEnemyKilled` _asbp_my_game_mode)
    (else
      (`self.K2_DestroyActor` _asbp_arrow)
      (`GameplayStatics.PlaySoundAtLocation` "/Game/Assets/Sounds/Arrow/arrow_1.arrow_1" (0.0 0.0 0.0) (struct) 0.1 1.0 0.0 null null null null))))

(event `OnShoot`
  (bind _returnvalue (`|SpawnActorFromClass` "/Game/Blueprints/Actor/Arrows/BP_Fireball.BP_Fireball_C" (`self.GetTransform`) "Undefined" "MultiplyWithRoot" null null))
  (set `/Game/Blueprints/Actor/Arrows/BP_Fireball.Damages` (`self.Damages`) _returnvalue))

(event `self.Sphere.OnComponentBeginOverlap`
  (params (OverlappedComponent :type "PrimitiveComponent Object Reference") (OtherActor :type "Actor Object Reference") (OtherComp :type "PrimitiveComponent Object Reference") (OtherBodyIndex :type Integer) (bFromSweep :type Boolean) (SweepResult :type "HitResult Structure (by ref)"))
  (if (== OtherActor (`self.CurrentTarget`))
    (set `self.LocationToStay` (`SceneComponent.K2_GetComponentLocation` (`self.CapsuleComponent`)))
    (set `self.StopSeeking` true)
    (bind _returnvalue (`KismetSystemLibrary.K2_SetTimerDelegate` (delegate `OnShoot`) 1.0 true))))

(event `self.Sphere.OnComponentEndOverlap`
  (params (OverlappedComponent :type "PrimitiveComponent Object Reference") (OtherActor :type "Actor Object Reference") (OtherComp :type "PrimitiveComponent Object Reference") (OtherBodyIndex :type Integer))
  (bind _troopdataasset (`self.TroopDataAsset`))
  (if (== OtherActor (`self.CurrentTarget`))
    (set `self.StopSeeking` false)
    (`KismetSystemLibrary.K2_ClearAndInvalidateTimerHandle` (stale `self.Sphere.OnComponentBeginOverlap` _returnvalue))
    (bind _asbp_my_aicontroller (cast `/Game/Blueprints/Core/BP_MyAIController` (`AIBlueprintHelperLibrary.GetAIController` (`self.GetController`))))
    (bind _target (`/Game/Blueprints/Core/BP_MyAIController.ChooseTarget` _asbp_my_aicontroller (`TroopData.FirstTypeTarget` _troopdataasset) (`TroopData.SecondTypeTarget` _troopdataasset) (`TroopData.ThirdTypeTarget` _troopdataasset)))
    (set `self.CurrentTarget` _target)))

(fn `UserConstructionScript`)