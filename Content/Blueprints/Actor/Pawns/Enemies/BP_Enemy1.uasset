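; BP_Enemy1 is an enemy pawn that takes its speed, health, damage and random money drop from a troop data asset.
; Each tick its AI controller moves it toward the closest target of three prioritized types, and it destroys itself below Z zero.
; Arrow overlaps damage it, and death pays the player and notifies the game mode.
; Crystal overlap starts a looping punch timer, cleared on any end overlap.
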(event `self.ReceiveBeginPlay`
  (bind _troopdataasset (`self.TroopDataAsset`))
  (set `CharacterMovementComponent.MaxWalkSpeed` (`TroopData.MovementSpeed` _troopdataasset) (`self.CharacterMovement`))
  (set `self.Health` (`TroopData.MaxHealth` _troopdataasset))
  (set `self.Damages` (`TroopData.Damages` _troopdataasset))
  (set `self.MoneyDrop` (`KismetMathLibrary.RandomIntegerInRange` (`TroopData.MinMoneyDrop` _troopdataasset) (`TroopData.MaxMoneyDrop` _troopdataasset))))

(event `self.ReceiveTick`
  (params (DeltaSeconds :type "Float (single-precision)"))
  (bind _troopdataasset (`self.TroopDataAsset`))
  (bind _asbp_my_aicontroller (cast `/Game/Blueprints/Core/BP_MyAIController` (`AIBlueprintHelperLibrary.GetAIController` (`self.GetController`))))
  (bind _target (`/Game/Blueprints/Core/BP_MyAIController.ChooseClosestTarget` _asbp_my_aicontroller (`TroopData.FirstTypeTarget` _troopdataasset) (`TroopData.SecondTypeTarget` _troopdataasset) (`TroopData.ThirdTypeTarget` _troopdataasset)))
  (`AIController.MoveToActor` _asbp_my_aicontroller _target -1.0 true true true null true)
  (if (< (.z (`SceneComponent.K2_GetComponentLocation` (`self.CapsuleComponent`))) 0.0)
    (`self.K2_DestroyActor`)))

(event `self.CapsuleComponent.OnComponentBeginOverlap`
  (params (OverlappedComponent :type "PrimitiveComponent Object Reference") (OtherActor :type "Actor Object Reference") (OtherComp :type "PrimitiveComponent Object Reference") (OtherBodyIndex :type Integer) (bFromSweep :type Boolean) (SweepResult :type "HitResult Structure (by ref)"))
  (bind _asbp_arrow (cast `/Game/Blueprints/Actor/Arrows/BP_Arrow` OtherActor)
    (:`then`
      (bind _output_get (set `self.Health` (- (`self.Health`) (`/Game/Blueprints/Actor/Arrows/BP_Arrow.Damages` _asbp_arrow))))
      (if (<= _output_get 0.0)
        (`self.K2_DestroyActor` _asbp_arrow)
        (`GameplayStatics.PlaySoundAtLocation` "/Game/Assets/Sounds/Arrow/arrow_2.arrow_2" (0.0 0.0 0.0) (struct) 0.1 1.0 0.0 null null null null)
        (bind _asbp_my_player_controller (cast `/Game/Blueprints/Core/BP_MyPlayerController` (`GameplayStatics.GetPlayerController` 0)))
        (set `/Game/Blueprints/Core/BP_MyPlayerController.Money` (+ (`/Game/Blueprints/Core/BP_MyPlayerController.Money` _asbp_my_player_controller) (`self.MoneyDrop`)) _asbp_my_player_controller)
        (`self.K2_DestroyActor`)
        (bind _asbp_my_game_mode (cast `/Game/Blueprints/Core/BP_MyGameMode` (`GameplayStatics.GetGameMode`)))
        (`/Game/Blueprints/Core/BP_MyGameMode.OnEnemyKilled` _asbp_my_game_mode)
        (else
          (`self.K2_DestroyActor` _asbp_arrow)
          (`GameplayStatics.PlaySoundAtLocation` "/Game/Assets/Sounds/Arrow/arrow_1.arrow_1" (0.0 0.0 0.0) (struct) 0.1 1.0 0.0 null null null null))))
    (:`CastFailed`
      (bind _asbp_crystal (cast `/Game/Blueprints/Actor/BP_Crystal` OtherActor))
      (bind _returnvalue (`KismetSystemLibrary.K2_SetTimerDelegate` (delegate `OnPunch`) 1.0 true)))))

(event `OnPunch`
  (set `/Game/Blueprints/Actor/BP_Crystal.Health` (- (`/Game/Blueprints/Actor/BP_Crystal.Health` (stale `self.CapsuleComponent.OnComponentBeginOverlap` _asbp_crystal)) (`self.Damages`)) (stale `self.CapsuleComponent.OnComponentBeginOverlap` _asbp_crystal))
  (`/Game/Blueprints/Actor/BP_Crystal.OnPunched` (stale `self.CapsuleComponent.OnComponentBeginOverlap` _asbp_crystal)))

(event `self.CapsuleComponent.OnComponentEndOverlap`
  (params (OverlappedComponent :type "PrimitiveComponent Object Reference") (OtherActor :type "Actor Object Reference") (OtherComp :type "PrimitiveComponent Object Reference") (OtherBodyIndex :type Integer))
  (`KismetSystemLibrary.K2_ClearAndInvalidateTimerHandle` (stale `self.CapsuleComponent.OnComponentBeginOverlap` _returnvalue)))

(fn `UserConstructionScript`)