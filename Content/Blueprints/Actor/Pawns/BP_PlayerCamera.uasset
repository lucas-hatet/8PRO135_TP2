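; BP_PlayerCamera is the player camera pawn, moved along the world X axis with scroll input.
; The ScrollUp and ScrollDown actions each restart their own timeline, whose vector track drives a per-update world offset on the root, with X scaled in opposite directions.
; Each update moves only while the root's X position is within that direction's fixed limit, without sweeping or clamping the final position.
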(event `InputAction|ScrollUp`
  (params (Key :type "Key Structure"))
  (:`Pressed`
    (bind (_direction _nouvelle_piste_0) (`Timeline|Chronologie` :!via `PlayFromStart`)
      (:`Update`
        (if (< (`KismetMathLibrary.BreakVector2D` (`KismetMathLibrary.Conv_VectorToVector2D` (`SceneComponent.K2_GetComponentLocation` (`self.DefaultSceneRoot`)))) 2000.0)
          (`SceneComponent.K2_AddWorldOffset` (`self.DefaultSceneRoot`) (`KismetMathLibrary.MakeVector` (* (.x _nouvelle_piste_0) 100.0) (.y _nouvelle_piste_0) (.z _nouvelle_piste_0)) false false))))))

(event `InputAction|ScrollDown`
  (params (Key :type "Key Structure"))
  (:`Pressed`
    (bind (_direction _nouvelle_piste_0) (`Timeline|Chronologie_0` :!via `PlayFromStart`)
      (:`Update`
        (if (> (`KismetMathLibrary.BreakVector2D` (`KismetMathLibrary.Conv_VectorToVector2D` (`SceneComponent.K2_GetComponentLocation` (`self.DefaultSceneRoot`)))) -5000.0)
          (`SceneComponent.K2_AddWorldOffset` (`self.DefaultSceneRoot`) (`KismetMathLibrary.MakeVector` (* (.x _nouvelle_piste_0) -100.0) (.y _nouvelle_piste_0) (.z _nouvelle_piste_0)) false false))))))

(fn `UserConstructionScript`)