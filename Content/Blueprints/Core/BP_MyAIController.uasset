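; AI controller Blueprint that supplies a ChooseTarget function for picking an actor to target.
; ChooseTarget tries three actor classes in priority order, falling through when a class is invalid or has no actors in the level.
; It returns a random actor from the first populated class, despite naming it ClosestTarget; no distance check is made.
; BeginPlay, Tick and the construction script contain no logic.
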(fn `ChooseTarget`
  (params (FirstTypeTarget :type "Actor Class Reference") (SecondTypeTarget :type "Actor Class Reference") (ThirdTypeTarget :type "Actor Class Reference"))
  (returns (Target :type "Actor Object Reference"))
  (locals (ClosestTarget :type "Actor Object Reference"))
  (if (`KismetSystemLibrary.IsValidClass` FirstTypeTarget)
    (bind _outactors (`GameplayStatics.GetAllActorsOfClass` FirstTypeTarget))
    (if (`KismetArrayLibrary.Array_IsNotEmpty` _outactors)
      (set `local.ClosestTarget` (`KismetArrayLibrary.Array_Random` _outactors))
      (return (`local.ClosestTarget`))
      (else
        (if (`KismetSystemLibrary.IsValidClass` SecondTypeTarget) :!label _label
          (bind _outactors_2 (`GameplayStatics.GetAllActorsOfClass` SecondTypeTarget))
          (if (`KismetArrayLibrary.Array_IsNotEmpty` _outactors_2)
            (set `local.ClosestTarget` (`KismetArrayLibrary.Array_Random` _outactors_2))
            (return (`local.ClosestTarget`))
            (else
              (if (`KismetSystemLibrary.IsValidClass` ThirdTypeTarget) :!label _label_2
                (bind _outactors_3 (`GameplayStatics.GetAllActorsOfClass` ThirdTypeTarget))
                (if (`KismetArrayLibrary.Array_IsNotEmpty` _outactors_3)
                  (set `local.ClosestTarget` (`KismetArrayLibrary.Array_Random` _outactors_3))
                  (return (`local.ClosestTarget`))))))
          (else
            (goto _label_2)))))
    (else
      (goto _label))))

(fn `UserConstructionScript`)