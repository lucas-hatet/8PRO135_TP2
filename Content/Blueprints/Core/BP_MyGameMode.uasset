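; BP_MyGameMode is the game mode that runs round-based waves through transition, preparation and assault phases via bound event dispatchers.
; Once the player controller is ready it starts a transition, which increments the round.
; Preparation runs a break timer that a skip event can cut short to start the assault.
; When a kill leaves the spawner finished and no enemy troops alive, it starts the next transition after a short delay.
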(event `self.ReceiveBeginPlay`
  (add `self.OnPreparationStart` (delegate `OnPreparationStart_Event`))
  (add `self.OnTransitionStart` (delegate `OnTransitionStartEvent`))
  (add `self.OnEnemyKilled` (delegate `OnEnemyKilled_Event`))
  (set `self.Round` 0)
  (bind _asbp_my_player_controller (cast `/Game/Blueprints/Core/BP_MyPlayerController` (`GameplayStatics.GetPlayerController` 0)))
  (add `/Game/Blueprints/Core/BP_MyPlayerController.OnPlayerControllerReady` _asbp_my_player_controller (delegate `OnPlayerControllerReady`)))

(event `OnPlayerControllerReady`
  (bind _asbp_my_player_controller (cast `/Game/Blueprints/Core/BP_MyPlayerController` (`GameplayStatics.GetPlayerController` 0)))
  (add `/Game/Blueprints/UI/WBP_InGame.OnWidgetReady` (`/Game/Blueprints/Core/BP_MyPlayerController.InGameWidgetRef` _asbp_my_player_controller) (delegate `OnWidgetReady`))
  (`self.OnTransitionStart`))

(event `OnWidgetReady`)

(event `OnPreparationStart_Event`
  (bind _returnvalue (`KismetSystemLibrary.K2_SetTimerDelegate` (delegate `OnAssaultStart_Event`) (`KismetMathLibrary.Conv_IntToDouble` (`self.BreakDuration`))))
  (add `self.OnPreparationSkip` (delegate `OnAssaultStart_Event`))
  (set `self.Timer` _returnvalue)
  (set `self.IsBreak` true))

(event `OnAssaultStart_Event`
  (`KismetSystemLibrary.K2_ClearAndInvalidateTimerHandle` (`self.Timer`))
  (set `self.IsBreak` false)
  (`self.OnAssaultStart`))

(event `OnTransitionStartEvent`
  (`/Engine/EditorBlueprintResources/StandardMacros.IncrementInt` (`self.Round`)))

(event `OnEnemyKilled_Event`
  (bind _returnvalue (`GameplayStatics.GetActorOfClass` "/Game/Blueprints/Actor/BP_Spawner.BP_Spawner_C"))
  (bind _outactors (`GameplayStatics.GetAllActorsOfClass` "/Script/PRO135_TP2.EnemyTroop"))
  (if (and (`/Game/Blueprints/Actor/BP_Spawner.SpawnFinished` _returnvalue) (`KismetArrayLibrary.Array_IsEmpty` _outactors))
    (`KismetSystemLibrary.Delay` 0.5)
    (`self.OnTransitionStart`)))

(fn `UserConstructionScript`)