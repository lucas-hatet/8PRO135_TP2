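; Player controller for a tower-based game that possesses the placed camera actor and enables mouse cursor, click and hover events.
; On the Game level it creates the in-game and tower info widgets and seeds Money and Troops from the game mode.
; The Pause input toggles a pause menu, saving and resuming the BreakTimer animation position.
; Buy deducts affordable costs or plays an error and signals insufficient coins; left click clears the selected tower.
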(event `self.ReceiveBeginPlay`
  (bind _returnvalue (`GameplayStatics.GetPlayerController` 0))
  (bind _outactors (`GameplayStatics.GetAllActorsOfClass` "/Game/Blueprints/Actor/Pawns/BP_PlayerCamera.BP_PlayerCamera_C"))
  (`self.Possess` _returnvalue (`|GetArrayItem` _outactors))
  (set `PlayerController.bShowMouseCursor` true _returnvalue)
  (set `PlayerController.bEnableClickEvents` true _returnvalue)
  (set `PlayerController.bEnableMouseOverEvents` true _returnvalue)
  (set `self.IsPaused` false)
  (bind _returnvalue_2 (`GameplayStatics.GetCurrentLevelName` true))
  (if (`BlueprintPathsLibrary.IsSamePath` _returnvalue_2 "Game")
    (bind _returnvalue_3 (`|CreateWidget` "/Game/Blueprints/UI/WBP_InGame.WBP_InGame_C"))
    (`UserWidget.AddToViewport` _returnvalue_3 0)
    (set `self.InGameWidgetRef` _returnvalue_3)
    (bind _asmy_game_mode (cast `MyGameMode` (`GameplayStatics.GetGameMode`)))
    (set `self.Money` (`MyGameMode.StartingMoney` _asmy_game_mode))
    (set `self.Troops` (`MyGameMode.StartingTroops` _asmy_game_mode))
    (`self.OnPlayerControllerReady`)
    (bind _returnvalue_4 (`|CreateWidget` "/Game/Blueprints/UI/WBP_TowerInfos.WBP_TowerInfos_C"))
    (`UserWidget.AddToViewport` _returnvalue_4 0)))

(event `InputAction|Pause`
  (params (Key :type "Key Structure"))
  (:`Pressed`
    (bind _returnvalue (`GameplayStatics.GetCurrentLevelName` true))
    (if (`BlueprintPathsLibrary.IsSamePath` _returnvalue "Game")
      (`self.TogglePause`))))

(event `Key|LeftMouseButton`
  (params (Key :type "Key Structure"))
  (:`Pressed`
    (set `self.TowerSelected` null)))

(fn `Buy`
  (params (Sum :type Integer))
  (returns (IsDone :type Boolean))
  (bind _asbp_my_player_controller (cast `/Game/Blueprints/Core/BP_MyPlayerController` (`GameplayStatics.GetPlayerController` 0)))
  (bind _returnvalue (- (`/Game/Blueprints/Core/BP_MyPlayerController.Money` _asbp_my_player_controller) Sum))
  (if (>= _returnvalue 0)
    (set `self.Money` _returnvalue)
    (return true)
    (else
      (`GameplayStatics.PlaySoundAtLocation` "/Game/Assets/Sounds/error.error" (0.0 0.0 0.0) (struct) 1.0 1.0 0.0 null null null null)
      (`self.OnNotEnoughCoins`)
      (return false))))

(fn `TogglePause`
  (bind _ingamewidgetref (`self.InGameWidgetRef`))
  (bind _pauseinstant (`self.PauseInstant`))
  (bind _breaktimer (`/Game/Blueprints/UI/WBP_InGame.BreakTimer` _ingamewidgetref))
  (if (`self.IsPaused`)
    (`Widget.RemoveFromParent` (`self.PauseWidgetRef`))
    (if (!= _pauseinstant 0.0)
      (`UserWidget.PlayAnimation` _ingamewidgetref _breaktimer _pauseinstant 1 "Forward" 1.0 false))
    (else
      (bind _returnvalue (`|CreateWidget` "/Game/Blueprints/UI/WBP_PauseMenu.WBP_PauseMenu_C"))
      (bind _output_get (set `self.PauseWidgetRef` _returnvalue))
      (`UserWidget.AddToViewport` _output_get 0)
      (bind _returnvalue_2 (`UserWidget.PauseAnimation` _ingamewidgetref _breaktimer))
      (set `self.PauseInstant` _returnvalue_2)))
  (bind _output_get_2 (set `self.IsPaused` (not (`self.IsPaused`))))
  (`GameplayStatics.SetGamePaused` _output_get_2))

(fn `UserConstructionScript`)